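; BP_Camera is an actor in PrincessDefense that checks whether its target actor lies within a forward-facing cone.
; Every Tick it takes the dot product of its forward vector and the normalized direction to the target, compared against a fixed threshold.
; The result sets the visibility of CameraComponent without propagating to children and is printed for debugging.
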(event `self.ReceiveTick`
  (params (DeltaSeconds :type "Float (single-precision)"))
  (bind _returnvalue (> (`KismetMathLibrary.Dot_VectorVector` (`self.GetActorForwardVector`) (`KismetMathLibrary.Normal` (- (`self.K2_GetActorLocation` (`self.ターゲット`)) (`self.K2_GetActorLocation`)))) 0.75))
  (`SceneComponent.SetVisibility` (`self.CameraComponent`) _returnvalue false)
  (`KismetSystemLibrary.PrintString` (`KismetStringLibrary.Conv_BoolToString` _returnvalue)))

(fn `UserConstructionScript`)